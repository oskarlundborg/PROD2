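; Car actor that picks its spawn location when play begins.
; Depending on flags, it uses its construction-time backup transform, a random point from the SpawnPositions actors, or a random XY inside one of four rectangular zones bounded by ZoneBeacons pairs at a fixed height.
; Random and fixed spawns also randomize yaw.
; Empty arrays log a message and fall back from zone to fixed spawns, then to the backup point.
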(event `self.ReceiveBeginPlay`
  (if (`self.ForceBackupSpawn`)
    (`self.SpawnOnBackup`)
    (elif (`self.RandomSpawnEnabled`)
      (`self.RandomSpawn`)
      (else
        (`self.FixedSpawns`)))))

(fn `FixedSpawns`
  (bind _spawnpositions (`self.SpawnPositions`))
  (if (<= (`KismetArrayLibrary.Array_Length` _spawnpositions) 0)
    (`KismetSystemLibrary.LogString` "No elements in SpawnPositions array, resorting to backup point.")
    (`self.SpawnOnBackup`)
    (else
      (`self.K2_SetActorLocation` (`self.K2_GetActorLocation` (`KismetArrayLibrary.Array_Random` _spawnpositions)))))
  (`self.K2_SetActorRotation` (`KismetMathLibrary.MakeRotator` 0.0 0.0 (`KismetMathLibrary.RandomFloatInRange` 0.0 360.0))))

(fn `RandomSpawn`
  (if (<= (`KismetArrayLibrary.Array_Length` (`self.ZoneBeacons`)) 0)
    (`KismetSystemLibrary.LogString` "No elements in ZoneBeacons array, resorting to FixedSpawns.")
    (`self.FixedSpawns`)
    (else
      (bind (_randomx _randomy) (`self.Zone`))
      (`self.K2_SetActorLocation` (`KismetMathLibrary.MakeVector` _randomx _randomy 60.0))
      (`self.K2_SetActorRotation` (`KismetMathLibrary.MakeRotator` 0.0 0.0 (`KismetMathLibrary.RandomFloatInRange` 0.0 360.0))))))

(fn `SpawnOnBackup`
  (bind _backupspawn_location (`KismetMathLibrary.BreakTransform` (`self.BackupSpawn`)))
  (`self.K2_SetActorLocation` _backupspawn_location))

(fn `UserConstructionScript`
  (set `self.BackupSpawn` (`self.GetTransform`)))

(fn `Zone`
  (returns (RandomX :type "Float (double-precision)") (RandomY :type "Float (double-precision)"))
  (locals (ReturnX :type "Float (double-precision)") (ReturnY :type "Float (double-precision)") (ZoneSelectionIndex :type Integer))
  (bind _zonebeacons (`self.ZoneBeacons`))
  (bind _zonebeacons_2 (`self.ZoneBeacons`))
  (bind _zonebeacons_3 (`self.ZoneBeacons`))
  (bind _zonebeacons_4 (`self.ZoneBeacons`))
  (bind _returnvalue (`self.GetTransform` (`|GetArrayItem` _zonebeacons)))
  (bind _returnvalue_2 (`self.GetTransform` (`|GetArrayItem` _zonebeacons 2)))
  (bind _returnvalue_3 (`self.GetTransform` (`|GetArrayItem` _zonebeacons_2 3)))
  (bind _returnvalue_4 (`self.GetTransform` (`|GetArrayItem` _zonebeacons_2 4)))
  (bind _returnvalue_5 (`self.GetTransform` (`|GetArrayItem` _zonebeacons_4 5)))
  (bind _returnvalue_6 (`self.GetTransform` (`|GetArrayItem` _zonebeacons_4 7)))
  (bind _returnvalue_7 (`self.GetTransform` (`|GetArrayItem` _zonebeacons_3 6)))
  (bind _returnvalue_8 (`self.GetTransform` (`|GetArrayItem` _zonebeacons_3 1)))
  (bind _output_get (set `local.ZoneSelectionIndex` (`KismetMathLibrary.RandomIntegerInRange` 0 3)))
  (switch `int` _output_get
    (:`0`
      (set `local.ReturnX` (`KismetMathLibrary.RandomFloatInRange` (.x (.location _returnvalue_2)) (.x (.location _returnvalue))))
      (set `local.ReturnY` (`KismetMathLibrary.RandomFloatInRange` (.y (.location _returnvalue_2)) (.y (.location _returnvalue)))))
    (:`1`
      (set `local.ReturnX` (`KismetMathLibrary.RandomFloatInRange` (.x (.location _returnvalue_3)) (.x (.location _returnvalue_4))))
      (set `local.ReturnY` (`KismetMathLibrary.RandomFloatInRange` (.y (.location _returnvalue_4)) (.y (.location _returnvalue_3)))))
    (:`2`
      (set `local.ReturnX` (`KismetMathLibrary.RandomFloatInRange` (.x (.location _returnvalue_5)) (.x (.location _returnvalue_6))))
      (set `local.ReturnY` (`KismetMathLibrary.RandomFloatInRange` (.y (.location _returnvalue_5)) (.y (.location _returnvalue_6)))))
    (:`3`
      (set `local.ReturnX` (`KismetMathLibrary.RandomFloatInRange` (.x (.location _returnvalue_7)) (.x (.location _returnvalue_8))))
      (set `local.ReturnY` (`KismetMathLibrary.RandomFloatInRange` (.y (.location _returnvalue_7)) (.y (.location _returnvalue_8))))))
  (return (`local.ReturnX`) (`local.ReturnY`)))