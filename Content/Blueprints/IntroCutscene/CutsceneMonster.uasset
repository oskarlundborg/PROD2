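; CutsceneMonster is the monster actor for the intro cutscene and supplies its sound effects through named custom events.
; FootstepEvent plays an attenuated footstep at the monster, then a louder, non-attenuated room shake at the player character's location.
; BreakInEvent plays an attenuated kill sound, then after a delay makes a second sound call with no sound assigned.
; RoarEvent and RummagingEvent are empty stubs.
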(event `FootstepEvent`
  (`GameplayStatics.PlaySoundAtLocation` "/Game/Sounds/Monster/Monster_Footstep.Monster_Footstep" (`self.K2_GetActorLocation` self) (struct) 1.0 1.0 0.0 "/Game/Sounds/CutsceneTracks/IntroMonsterAttenuation.IntroMonsterAttenuation" null null null)
  (`GameplayStatics.PlaySoundAtLocation` "/Game/Sounds/CutsceneTracks/Room_Shake.Room_Shake" (`self.K2_GetActorLocation` (`GameplayStatics.GetPlayerCharacter` 0)) (struct) 4.0 1.0 0.0 null null null null))

(event `BreakInEvent`
  (bind _returnvalue (`self.K2_GetActorLocation` self))
  (`GameplayStatics.PlaySoundAtLocation` "/Game/Sounds/Monster/MonsterKillPlayer1.MonsterKillPlayer1" _returnvalue (struct) 1.0 1.0 0.0 "/Game/Sounds/CutsceneTracks/IntroMonsterAttenuation.IntroMonsterAttenuation" null null null)
  (`KismetSystemLibrary.Delay` 1.0)
  (`GameplayStatics.PlaySoundAtLocation` null _returnvalue (struct) 1.0 1.0 0.0 "/Game/Sounds/CutsceneTracks/IntroMonsterAttenuation.IntroMonsterAttenuation" null null null))

(event `RoarEvent`)

(event `RummagingEvent`)

(fn `UserConstructionScript`)