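; BP_Enemy is a monster that gives audio and controller rumble cues, and plays a kill sound once when its capsule overlaps the first-person player.
; Tick scales force feedback by proximity to the player and makes the growl audible only while moving horizontally.
; While moving, a downward trace picks footsteps by surface type, paced by Delay nodes and faster on default surfaces when Chasing.
; Grass and Concrete footsteps have no sound assigned.
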(event `self.ReceiveTick`
  (params (DeltaSeconds :type "Float (single-precision)"))
  (bind _returnvalue (`self.K2_GetActorLocation`))
  (bind (_velocity_x _velocity_y) (`KismetMathLibrary.BreakVector` (`MovementComponent.Velocity` (`self.CharacterMovement`))))
  (`ForceFeedbackComponent.SetIntensityMultiplier` (`self.ForceFeedback`) (- 1.0 (`KismetMathLibrary.FClamp` (/ (`KismetMathLibrary.Vector_Distance` (`self.K2_GetActorLocation` self) (`self.K2_GetActorLocation` (`self.Player`))) 1000.0))))
  (if (or (!= _velocity_x 0.0) (!= _velocity_y 0.0))
    (`AudioComponent.SetVolumeMultiplier` (`self.Growl_0`) 1.0)
    (bind (_outhit _returnvalue_2) (`KismetSystemLibrary.LineTraceSingle` _returnvalue (- _returnvalue (0.0 0.0 150.0)) "TraceTypeQuery1"))
    (if _returnvalue_2
      (switch `EPhysicalSurface` (`GameplayStatics.GetSurfaceType` _outhit)
        (:`SurfaceType_Default`
          (if (`self.Chasing`)
            (`KismetSystemLibrary.Delay` 0.4)
            (else
              (`KismetSystemLibrary.Delay` 0.8)))
          (bind (_bblockinghit _binitialoverlap _time _distance _location) (`GameplayStatics.BreakHitResult` _outhit))
          (`GameplayStatics.PlaySoundAtLocation` "/Game/Sounds/Monster/SQ_FootstepDefaultMonster.SQ_FootstepDefaultMonster" _location (struct) 1.0 1.0 0.0 "/Game/Sounds/enemy.enemy" null null null))
        (:`SurfaceType2`
          (`KismetSystemLibrary.Delay` 0.8)
          (`GameplayStatics.PlaySoundAtLocation` null _location (struct) 1.0 1.0 0.0 "/Game/Sounds/enemy.enemy" null null null))
        (:`SurfaceType9`
          (`KismetSystemLibrary.Delay` 0.8)
          (`GameplayStatics.PlaySoundAtLocation` null _location (struct) 1.0 1.0 0.0 "/Game/Sounds/enemy.enemy" null null null))))
    (else
      (`AudioComponent.SetVolumeMultiplier` (`self.Growl_0`) 0.0))))

(event `self.ReceiveBeginPlay`
  (`ForceFeedbackComponent.SetIntensityMultiplier` (`self.ForceFeedback`) 0.0)
  (bind _returnvalue (`GameplayStatics.GetActorOfClass` "/Game/FirstPerson/Blueprints/BP_FirstPersonCharacter.BP_FirstPersonCharacter_C"))
  (set `self.Player` _returnvalue))

(event `self.Capsule.OnComponentBeginOverlap`
  (params (OverlappedComponent :type "PrimitiveComponent Object Reference") (OtherActor :type "Actor Object Reference") (OtherComp :type "PrimitiveComponent Object Reference") (OtherBodyIndex :type Integer) (bFromSweep :type Boolean) (SweepResult :type "HitResult Structure (by ref)"))
  (cast `/Game/FirstPerson/Blueprints/BP_FirstPersonCharacter` OtherActor)
  (`/Engine/EditorBlueprintResources/StandardMacros.DoOnce` false
    (:`Completed`
      (`GameplayStatics.PlaySound2D` "/Game/Sounds/Monster/MonsterKillPlayer1.MonsterKillPlayer1" 0.6 1.0 0.0 null null))))

(fn `UserConstructionScript`)