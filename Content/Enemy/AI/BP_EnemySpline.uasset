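; BP_EnemySpline is a patrol route that supplies spline points for an enemy to follow.
; GetSplinePointPosition returns the world location of the spline point at the current patrol index.
; IncrementPatrolRoute steps that index by a direction that flips at the last and first points, so the route runs back and forth.
; Tick only prints a leftover debug string every frame.
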(event `self.ReceiveTick`
  (params (DeltaSeconds :type "Float (single-precision)"))
  (`KismetSystemLibrary.PrintString` "DOES SPLINE EXIST?!?!!"))

(event `IncrementPatrolRoute`
  ;[1 1 1] Increments patrol index for the enemy based on which point on the spline it currently is until it reaches the last point (-1 is going backwards and 1 is going forwards)
  (bind _output_get (set `self.PatrolIndex` (+ (`self.PatrolIndex`) (`self.Direction`))))
  (if (== _output_get (- (`SplineComponent.GetNumberOfSplinePoints` (`self.PatrolRoute`)) 1))
    (set `self.Direction` -1)
    (elif (== (`self.PatrolIndex`) 0)
      (set `self.Direction` 1))))

(fn `GetSplinePointPosition`
  (returns (Position :type "Vector Structure"))
  (return (`SplineComponent.GetLocationAtSplinePoint` (`self.PatrolRoute`) (`self.PatrolIndex`) "World")))

(fn `UserConstructionScript`)