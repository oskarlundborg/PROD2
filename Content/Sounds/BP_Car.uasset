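; BP_Car is an actor that places itself at a random or fixed spawn location on BeginPlay, at a constant height.
; In random mode, coin flips pick one of four beacon-bounded zones, and disabled zones cascade toward Zone1, then to FixedSpawnPoints.
; Fixed mode draws from SpawnLocations, and both modes randomize yaw.
; An empty beacon or location array triggers EmergencySpawn at the BackupSpawn position, without changing rotation.
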(event `self.ReceiveBeginPlay`
  (if (`self.RandomSpawnEnabled`)
    (`self.RandomSpawn`)
    (else
      (`self.FixedSpawnPoints`))))

(fn `EmergencySpawn`
  (bind _backupspawn (`self.BackupSpawn`))
  (`self.K2_SetActorLocation` (`KismetMathLibrary.MakeVector` (.x (.location _backupspawn)) (.y (.location _backupspawn)) 95.0)))

(fn `FixedSpawnPoints`
  (bind (_returnvalue_x _returnvalue_y) (`KismetMathLibrary.BreakVector` (`self.K2_GetActorLocation` (`|GetArrayItem` (`self.SpawnLocations`) (`KismetMathLibrary.RandomInteger` (`self.MaxIndex`))))))
  (if (<= (`KismetArrayLibrary.Array_Length` (`self.SpawnLocations`)) 0)
    (`self.EmergencySpawn`)
    (else
      (bind _output_get (set `self.MaxIndex` (- (`KismetArrayLibrary.Array_Length` (`self.SpawnLocations`)) 1)))
      (if (<= _output_get 0)
        (set `self.MaxIndex` 0))
      (`self.K2_SetActorLocation` (`KismetMathLibrary.MakeVector` _returnvalue_x _returnvalue_y 95.0))
      (`self.K2_SetActorRotation` (`KismetMathLibrary.MakeRotator` 0.0 0.0 (`KismetMathLibrary.RandomFloatInRange` 0.0 360.0))))))

(fn `RandomSpawn`
  (if (<= (`KismetArrayLibrary.Array_Length` (`self.ZoneBeacons`)) 0)
    (`self.EmergencySpawn`)
    (elif (`KismetMathLibrary.RandomBool`)
      (if (`KismetMathLibrary.RandomBool`)
        (if (`self.ZoneEnabled_4`)
          (bind (_randomx_z4 _randomy_z4) (`self.Zone4`))
          (`self.K2_SetActorLocation` (`KismetMathLibrary.MakeVector` _randomx_z4 _randomy_z4 95.0))
          (`self.K2_SetActorRotation` (`KismetMathLibrary.MakeRotator` 0.0 0.0 (`KismetMathLibrary.RandomFloatInRange` 0.0 360.0)) :!label _label)
          (else
            (if (`self.ZoneEnabled_3`) :!label _label_2
              (bind (_randomx_z3 _randomy_z3) (`self.Zone3`))
              (`self.K2_SetActorLocation` (`KismetMathLibrary.MakeVector` _randomx_z3 _randomy_z3 95.0))
              (goto _label)
              (else
                (if (`self.ZoneEnabled_2`) :!label _label_3
                  (bind (_randomx_z1 _randomy_z1) (`self.Zone2`))
                  (`self.K2_SetActorLocation` (`KismetMathLibrary.MakeVector` _randomx_z1 _randomy_z1 95.0))
                  (goto _label)
                  (else
                    (if (`self.ZoneEnabled_1`) :!label _label_4
                      (bind (_randomx_z2 _randomy_z2) (`self.Zone1`))
                      (`self.K2_SetActorLocation` (`KismetMathLibrary.MakeVector` _randomx_z2 _randomy_z2 95.0))
                      (goto _label)
                      (else
                        (`self.FixedSpawnPoints`)))))))))
        (else
          (goto _label_2)))
      (elif (`KismetMathLibrary.RandomBool`)
        (goto _label_3)
        (else
          (goto _label_4))))))

(fn `UserConstructionScript`)

(fn `Zone1`
  (returns (RandomX_Z2 :type "Float (double-precision)") (RandomY_Z2 :type "Float (double-precision)"))
  (bind _zonebeacons (`self.ZoneBeacons`))
  (bind _returnvalue (`self.GetTransform` (`|GetArrayItem` _zonebeacons)))
  (bind _returnvalue_2 (`self.GetTransform` (`|GetArrayItem` _zonebeacons 2)))
  (return (`KismetMathLibrary.RandomFloatInRange` (.x (.location _returnvalue_2)) (.x (.location _returnvalue))) (`KismetMathLibrary.RandomFloatInRange` (.y (.location _returnvalue_2)) (.y (.location _returnvalue)))))

(fn `Zone2`
  (returns (RandomX_Z1 :type "Float (double-precision)") (RandomY_Z1 :type "Float (double-precision)"))
  (bind _zonebeacons (`self.ZoneBeacons`))
  (bind _returnvalue (`self.GetTransform` (`|GetArrayItem` _zonebeacons 3)))
  (bind _returnvalue_2 (`self.GetTransform` (`|GetArrayItem` _zonebeacons 4)))
  (return (`KismetMathLibrary.RandomFloatInRange` (.x (.location _returnvalue)) (.x (.location _returnvalue_2))) (`KismetMathLibrary.RandomFloatInRange` (.y (.location _returnvalue_2)) (.y (.location _returnvalue)))))

(fn `Zone3`
  (returns (RandomX_Z3 :type "Float (double-precision)") (RandomY_Z3 :type "Float (double-precision)"))
  (bind _zonebeacons (`self.ZoneBeacons`))
  (bind _returnvalue (`self.GetTransform` (`|GetArrayItem` _zonebeacons 7)))
  (bind _returnvalue_2 (`self.GetTransform` (`|GetArrayItem` _zonebeacons 5)))
  (return (`KismetMathLibrary.RandomFloatInRange` (.x (.location _returnvalue_2)) (.x (.location _returnvalue))) (`KismetMathLibrary.RandomFloatInRange` (.y (.location _returnvalue)) (.y (.location _returnvalue_2)))))

(fn `Zone4`
  (returns (RandomX_Z4 :type "Float (double-precision)") (RandomY_Z4 :type "Float (double-precision)"))
  (bind _zonebeacons (`self.ZoneBeacons`))
  (bind _returnvalue (`self.GetTransform` (`|GetArrayItem` _zonebeacons 6)))
  (bind _returnvalue_2 (`self.GetTransform` (`|GetArrayItem` _zonebeacons 1)))
  (return (`KismetMathLibrary.RandomFloatInRange` (.x (.location _returnvalue_2)) (.x (.location _returnvalue))) (`KismetMathLibrary.RandomFloatInRange` (.y (.location _returnvalue)) (.y (.location _returnvalue_2)))))