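; Enemy monster that hunts the player, with surface-aware footsteps, proximity force feedback and a kill on capsule overlap.
; Tick traces downward to pick sand, grass, water or mud foley macros, which set walk speed by AI state and time footsteps with Delays.
; BeginPlay loads base speed and AI sight radius from a parameter file.
; Player overlap disables input, logs elapsed time to a file and opens PauseMenu after a delay.
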(event `self.ReceiveTick`
  (params (DeltaSeconds :type "Float (single-precision)"))
  (bind _returnvalue (`self.K2_GetActorLocation`))
  (bind _defaultenemyspeed (`self.DefaultEnemySpeed`))
  (bind _charactermovement (`self.CharacterMovement`))
  (bind _defaultenemyspeed_2 (`self.DefaultEnemySpeed`))
  (bind _charactermovement_2 (`self.CharacterMovement`))
  (bind _defaultenemyspeed_3 (`self.DefaultEnemySpeed`))
  (bind _charactermovement_3 (`self.CharacterMovement`))
  (bind _defaultenemyspeed_4 (`self.DefaultEnemySpeed`))
  (bind _charactermovement_4 (`self.CharacterMovement`))
  (bind _ispatroling (`self.IsPatroling`))
  (bind _ischasingtarget (`self.IsChasingTarget`))
  (bind _iswalkingtowardstarget (`self.IsWalkingTowardsTarget`))
  (bind (_velocity_x _velocity_y) (`KismetMathLibrary.BreakVector` (`MovementComponent.Velocity` (`self.CharacterMovement`))))
  (`|ExecutionSequence`
    (:`then_0`
      (if (or (!= _velocity_x 0.0) (!= _velocity_y 0.0))
        (bind (_outhit _returnvalue_2) (`KismetSystemLibrary.LineTraceSingle` _returnvalue (- _returnvalue (0.0 0.0 150.0)) "TraceTypeQuery1"))
        (if _returnvalue_2
          (switch `EPhysicalSurface` (`GameplayStatics.GetSurfaceType` _outhit)
            (:`SurfaceType1`
              ;[1 1 1] Foley Logic and SoundTriggers
              (if _ischasingtarget
                (set `CharacterMovementComponent.MaxWalkSpeed` _defaultenemyspeed _charactermovement)
                (`KismetSystemLibrary.Delay` 0.3)
                (bind (_bblockinghit _binitialoverlap _time _distance _location) (`GameplayStatics.BreakHitResult` _outhit))
                (`GameplayStatics.PlaySoundAtLocation` "/Game/Sounds/Monster/Footsteps/Sand/SQ_MonsterFootstepSand.SQ_MonsterFootstepSand" _location (struct) 0.85 1.0 0.0 null null null null :!label _label)
                (elif _iswalkingtowardstarget
                  (set `CharacterMovementComponent.MaxWalkSpeed` (- _defaultenemyspeed 323.0) _charactermovement)
                  (`KismetSystemLibrary.Delay` 0.8)
                  (goto _label)
                  (elif _ispatroling
                    (set `CharacterMovementComponent.MaxWalkSpeed` (- _defaultenemyspeed 100.0) _charactermovement)
                    (`KismetSystemLibrary.Delay` 0.5)
                    (goto _label)))))
            (:`SurfaceType2`
              (if _ischasingtarget
                (set `CharacterMovementComponent.MaxWalkSpeed` _defaultenemyspeed_2 _charactermovement_2)
                (`KismetSystemLibrary.Delay` 0.3)
                (`GameplayStatics.PlaySoundAtLocation` "/Game/Sounds/Monster/Footsteps/Grass/SQ_MonsterFootstepGrass.SQ_MonsterFootstepGrass" _location (struct) 1.25 1.0 0.0 null null null null :!label _label_2)
                (elif _iswalkingtowardstarget
                  (set `CharacterMovementComponent.MaxWalkSpeed` (- _defaultenemyspeed_2 323.0) _charactermovement_2)
                  (`KismetSystemLibrary.Delay` 0.8)
                  (goto _label_2)
                  (elif _ispatroling
                    (set `CharacterMovementComponent.MaxWalkSpeed` (- _defaultenemyspeed_2 100.0) _charactermovement_2)
                    (`KismetSystemLibrary.Delay` 0.5)
                    (goto _label_2)))))
            (:`SurfaceType3`
              (if _ischasingtarget
                (set `CharacterMovementComponent.MaxWalkSpeed` (- _defaultenemyspeed_3 400.0) _charactermovement_3)
                (`KismetSystemLibrary.Delay` 0.3)
                (`GameplayStatics.PlaySoundAtLocation` "/Game/Sounds/Monster/Footsteps/Water/SQ_MonsterFootstepWater.SQ_MonsterFootstepWater" _location (struct) 1.0 1.0 0.0 null null null null :!label _label_3)
                (elif _iswalkingtowardstarget
                  (set `CharacterMovementComponent.MaxWalkSpeed` (- _defaultenemyspeed_3 573.0) _charactermovement_3)
                  (`KismetSystemLibrary.Delay` 0.8)
                  (goto _label_3)
                  (elif _ispatroling
                    (set `CharacterMovementComponent.MaxWalkSpeed` (- _defaultenemyspeed_3 500.0) _charactermovement_3)
                    (`KismetSystemLibrary.Delay` 0.5)
                    (goto _label_3)))))
            (:`SurfaceType4`
              (if _ischasingtarget
                (set `CharacterMovementComponent.MaxWalkSpeed` (- _defaultenemyspeed_4 300.0) _charactermovement_4)
                (`KismetSystemLibrary.Delay` 0.3)
                (`GameplayStatics.PlaySoundAtLocation` "/Game/Sounds/Monster/Footsteps/Mud/SQ_MonsterFootstepMud.SQ_MonsterFootstepMud" _location (struct) 0.85 1.0 0.0 null null null null :!label _label_4)
                (elif _iswalkingtowardstarget
                  (set `CharacterMovementComponent.MaxWalkSpeed` (- _defaultenemyspeed_4 523.0) _charactermovement_4)
                  (`KismetSystemLibrary.Delay` 0.85)
                  (goto _label_4)
                  (elif _ispatroling
                    (set `CharacterMovementComponent.MaxWalkSpeed` (- _defaultenemyspeed_4 400.0) _charactermovement_4)
                    (`KismetSystemLibrary.Delay` 0.6)
                    (goto _label_4)))))))))
    (:`then_1`
      (bind _outactors (`GameplayStatics.GetAllActorsWithTag` (`self.Prey`)))
      (`ForceFeedbackComponent.SetIntensityMultiplier` (`self.ForceFeedback`) (- 0.65 (`KismetMathLibrary.FClamp` (/ (`KismetMathLibrary.Vector_Distance` (`self.K2_GetActorLocation` self) (`self.K2_GetActorLocation` (`|GetArrayItem` _outactors))) 1000.0) 0.0 0.65))))))

(event `self.ReceiveBeginPlay`
  (bind _readwritefiles (`self.ReadWriteFiles`))
  (set `self.StartTime` (`KismetMathLibrary.Now`))
  (`ReadWriteFilesComponent.ReadFile` _readwritefiles "EnemyParameters.txt")
  (set `self.DefaultEnemySpeed` (`KismetStringLibrary.Conv_StringToDouble` (`ReadWriteFilesComponent.ParameterOne` _readwritefiles)))
  (bind _asaic_enemy (cast `/Game/Enemy/AI/AIC_Enemy` (`AIBlueprintHelperLibrary.GetAIController` self))
    (:`then`
      (set `PawnSensingComponent.SightRadius` (`KismetStringLibrary.Conv_StringToDouble` (`ReadWriteFilesComponent.ParameterTwo` _readwritefiles)) (`/Game/Enemy/AI/AIC_Enemy.PawnSensing` _asaic_enemy)))
    (:`CastFailed`
      _))
  (`ForceFeedbackComponent.SetIntensityMultiplier` (`self.ForceFeedback`) 0.0)
  (bind _returnvalue (`GameplayStatics.GetActorOfClass` "/Game/FirstPerson/Blueprints/BP_FirstPersonCharacter.BP_FirstPersonCharacter_C"))
  (set `self.Player` _returnvalue)
  (`AudioComponent.Play` (`self.CaughtPlayer`) 0.0)
  (`AudioComponent.Play` (`self.Growl_0`) 0.0))

(event `self.Capsule.OnComponentBeginOverlap`
  (params (OverlappedComponent :type "PrimitiveComponent Object Reference") (OtherActor :type "Actor Object Reference") (OtherComp :type "PrimitiveComponent Object Reference") (OtherBodyIndex :type Integer) (bFromSweep :type Boolean) (SweepResult :type "HitResult Structure (by ref)"))
  (bind _returnvalue (`GameplayStatics.GetPlayerController` 0))
  (bind _playercharacter (`self.PlayerCharacter`))
  (bind _asbp_first_person_character (cast `/Game/FirstPerson/Blueprints/BP_FirstPersonCharacter` OtherActor))
  (`/Engine/EditorBlueprintResources/StandardMacros.DoOnce` false
    (:`Completed`
      (bind _output_get (set `self.PlayerCharacter` _asbp_first_person_character))
      (set `/Game/FirstPerson/Blueprints/BP_FirstPersonCharacter.NoResume` true _output_get)
      (`GameplayStatics.PlaySound2D` "/Game/Sounds/Monster/KillSound/Kill_3_Ape.Kill_3_Ape" 0.2 1.0 0.0 null null)
      (`AudioComponent.SetVolumeMultiplier` (`self.Growl_0`) 0.0)
      (set `self.ElapsedTime` (`KismetMathLibrary.Now`))
      (`ReadWriteFilesComponent.WriteToFile` (`self.ReadWriteFiles`) "EventLog.txt" (`KismetStringLibrary.Concat_StrStr` (`KismetStringLibrary.Conv_DoubleToString` (`KismetMathLibrary.GetTotalSeconds` (- (`KismetMathLibrary.GetTimeOfDay` (`self.ElapsedTime`)) (`KismetMathLibrary.GetTimeOfDay` (`self.StartTime`))))) " Seconds Elapsed, Player Died."))
      (`self.DisableInput` _playercharacter _returnvalue)
      (set `/Game/FirstPerson/Blueprints/BP_FirstPersonCharacter.CanOpenMenu` false _playercharacter)
      (`KismetSystemLibrary.Delay` 4.0)
      (bind _returnvalue_2 (`|CreateWidget` "/Game/Blueprints/Menu/WidgetBlueprint/PauseMenu.PauseMenu_C" _returnvalue))
      (`UserWidget.AddToViewport` _returnvalue_2 0)
      (set `PlayerController.bShowMouseCursor` true _returnvalue)
      (`WidgetBlueprintLibrary.SetInputMode_GameAndUIEx` _returnvalue null)
      (`AudioComponent.Stop` (`self.Growl_0`))
      (`AudioComponent.Stop` (`self.CaughtPlayer`))
      (set `self.PlayerDead` true))))

(fn `UserConstructionScript`)